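; BP_Character_Jamchu is the Jamchu character Blueprint in SmashUE, built around a StateMachine component and still holding test logic.
; Shortly after BeginPlay it binds an event to the state machine's change notification, and the OnChangedState handler switches on the state ID without any actions.
; The H key forces the Jump state and Tick prints a debug string, while the Walk and Idle changes are disconnected.
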(event Custom|OnChangedState
  (params (StateID :type ESmashCharacterStateID%20Enum :default "None"))
  (switch Utilities|FlowControl|Switch|SwitchonESmashCharacterStateID StateID))

(event EventBeginPlay
  ;[1 1 1] Begin Play
  (Utilities|FlowControl|Delay 0.2)
  (EventDispatchers|BindEventtoOnChangedState (Variables|Default|GetStateMachine) (EventDispatchers|CreateEvent :!event Custom|OnChangedState)))

(event EventTick
  (params (DeltaSeconds :type Float%20%28single-precision%29))
  (Development|PrintString "Hello"))

(event Input|KeyboardEvents|H
  (params (Key :type Key%20Structure :default "None"))
  (:Pressed
    (Class|SmashCharacterStateMachine|ChangeState (Variables|Default|GetStateMachine) "Jump")))

(event Input|KeyboardEvents|F
  (params (Key :type Key%20Structure :default "None")))

(event Input|KeyboardEvents|G
  (params (Key :type Key%20Structure :default "None")))

(fn ConstructionScript)